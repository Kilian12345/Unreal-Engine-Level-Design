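; BP_Watcher is an AI enemy that destroys any Player-tagged actor it hits while its PlayerSpotted flag is false.
; A DashingToPlayer function casts to BP_PlayerCharacter and halts that character's movement; nothing in this file calls it.
; Nodes that would disable the player's dash and set PlayerSpotted are disconnected, so they never run.
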(event EventBeginPlay)

(event Collision|EventActorBeginOverlap
  (params (OtherActor :type Actor%20Object%20Reference)))

(event EventTick
  (params (DeltaSeconds :type Float%20%28single-precision%29)))

(event Collision|EventHit
  (params (MyComp :type Primitive%20Component%20Object%20Reference) (Other :type Actor%20Object%20Reference) (OtherComp :type Primitive%20Component%20Object%20Reference) (bSelfMoved :type Boolean) (HitLocation :type Vector :default "0, 0, 0") (HitNormal :type Vector :default "0, 0, 0") (NormalImpulse :type Vector :default "0, 0, 0") (Hit :type Hit%20Result%20Structure%20%28by%20ref%29))
  (if (and (Actor|ActorHasTag Other "Player") (not (Variables|Default|GetPlayerSpotted)))
    (Actor|DestroyActor Other)))

(fn ConstructionScript)

(fn DashingtoPlayer
  (bind _asbp_player_character (Utilities|Casting|CastToBP_PlayerCharacter (Game|GetPlayerCharacter 0)))
  (Components|Movement|StopMovementImmediately (Variables|/Script/Engine.Character|GetCharacterMovement _asbp_player_character))
  (Class|NavMovementComponent|StopActiveMovement (Variables|/Script/Engine.Character|GetCharacterMovement _asbp_player_character)))