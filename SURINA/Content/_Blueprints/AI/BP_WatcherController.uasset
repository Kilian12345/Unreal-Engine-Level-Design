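; AI controller for the Watcher that runs BT_Watcher and feeds it player sight data through the Blackboard.
; On sensing a Player-tagged actor, perception cancels EnemyTimer, sets PlayerLineOfSight and writes PlayerLocation, which Tick also refreshes from the perceived actor.
; Other perception updates start a LineOfSightTimer delay that clears line of sight and calls SetValueAsObject with no value on PlayerLocation, despite it being a vector key.
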(event OnTargetPerceptionUpdated(AIPerception)
  (params (Actor :type Actor%20Object%20Reference) (Stimulus :type AI%20Stimulus%20Structure))
  (bind _blackboard (Variables|Default|GetBlackboard))
  (if (and (Actor|ActorHasTag Actor "Player") (.bSuccessfullySensed (Utilities|Struct|BreakAIStimulus Stimulus)))
    (Utilities|Time|ClearandInvalidateTimerbyHandle (Variables|Default|GetEnemyTimer))
    (AI|Components|Blackboard|SetValueasBool _blackboard (Variables|Default|GetPlayerLineOfSight) true)
    (AI|Components|Blackboard|SetValueasVector _blackboard (Variables|Default|GetPlayerLocation) (Transformation|GetActorLocation Actor))
    (else
      ;[1 1 1] okaou
      (bind _returnvalue (Utilities|Time|SetTimerbyEvent (delegate Custom|StartEnemyTimer) (Variables|Default|GetLineOfSightTimer)))
      (Variables|Default|SetEnemyTimer _returnvalue))))

(event Custom|StartEnemyTimer
  (bind _blackboard (Variables|Default|GetBlackboard))
  ;[1 1 1] okaou
  (AI|Components|Blackboard|SetValueasBool _blackboard (Variables|Default|GetPlayerLineOfSight) false)
  (AI|Components|Blackboard|SetValueasObject _blackboard (Variables|Default|GetPlayerLocation) 0))

(event EventBeginPlay)

(event EventTick
  (params (DeltaSeconds :type Float%20%28single-precision%29))
  (AI|Components|Blackboard|SetValueasVector (Variables|Default|GetBlackboard) (Variables|Default|GetPlayerLocation) (Transformation|GetActorLocation (stale OnTargetPerceptionUpdated(AIPerception) Actor))))

(event EventPossess
  (params (PossessedPawn :type Pawn%20Object%20Reference))
  (AI|RunBehaviorTree "/Game/_Blueprints/AI/BT_Watcher.BT_Watcher"))

(fn ConstructionScript)